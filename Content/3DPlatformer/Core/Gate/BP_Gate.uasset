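; BP_Gate is a key-locked forcefield gate for the 3D platformer that opens for a player carrying a matching key.
; On BeginPlay it gives the forcefield mesh a dynamic material tinted with the gate's color.
; When BP_MainCharacter enters the trigger box, its Keys tag container is tested against the GateType query.
; A match runs a timeline that animates forcefield opacity, with mesh collision disabled after a short delay.
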(event OnComponentBeginOverlap(Box)
  (params (OverlappedComponent :type Primitive%20Component%20Object%20Reference) (OtherActor :type Actor%20Object%20Reference) (OtherComp :type Primitive%20Component%20Object%20Reference) (OtherBodyIndex :type Integer) (bFromSweep :type Boolean) (SweepResult :type Hit%20Result%20Structure%20%28by%20ref%29))
  (bind _asbp_main_character (Utilities|Casting|CastToBP_MainCharacter OtherActor))
  (if (GameplayTags|DoesContainerMatchTagQuery (Variables|/Game/3DPlatformer/Core/Player/BP_MainCharacter.BP_MainCharacter_C|GetKeys _asbp_main_character) (Variables|Default|GetGateType))
    (CallFunction|OpenGate)))

(event Custom|OpenGate
  (bind _opacity (Timeline|Timeline Play)
    (:Update
      (Rendering|Material|SetScalarParameterValue (Variables|Default|GetForceFieldMatRef) "Opacity" _opacity :!class /Script/Engine.MaterialInstanceDynamic)
      (Utilities|FlowControl|Delay 0.7)
      (Collision|SetCollisionEnabled (Variables|Default|GetSM_Forcefield) "NoCollision"))))

(event EventBeginPlay
  (bind _returnvalue (Rendering|Material|CreateDynamicMaterialInstance (Variables|Default|GetSM_Forcefield) 0 "/Game/TeachersMarketplace/Assets/Architecture/Gate/Material/MI_forcefield.MI_forcefield" "None" :!class /Script/Engine.PrimitiveComponent))
  (Variables|Default|SetForceFieldMatRef _returnvalue)
  (Rendering|Material|SetVectorParameterValue (Variables|Default|GetForceFieldMatRef) "ColorMultiplier" (Variables|Default|GetColorForcefield) :!class /Script/Engine.MaterialInstanceDynamic))

(event Collision|EventActorBeginOverlap
  (params (OtherActor :type Actor%20Object%20Reference)))

(event EventTick
  (params (DeltaSeconds :type Float%20%28single-precision%29)))

(fn ConstructionScript)