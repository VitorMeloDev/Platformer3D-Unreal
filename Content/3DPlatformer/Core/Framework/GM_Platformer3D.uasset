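; Game mode for a 3D platformer that tracks the player's respawn point and handles winning.
; On BeginPlay it takes the level's PlayerStart transform as the initial respawn point.
; UpdateRespawPoint resets the previous checkpoint to normal, then stores the new transform and checkpoint reference.
; The WinTheGame event casts the player character to BP_MainCharacter and triggers its celebration.
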(event Custom|WinTheGame
  (bind _asbp_main_character (Utilities|Casting|CastToBP_MainCharacter (Game|GetPlayerCharacter 0)))
  (Default|Celebration _asbp_main_character))

(event EventBeginPlay
  (bind _returnvalue (Actor|GetActorOfClass "/Script/Engine.PlayerStart"))
  (Variables|Default|SetRespawPoint (Transformation|GetActorTransform _returnvalue)))

(event EventTick
  (params (DeltaSeconds :type Float%20%28single-precision%29)))

(fn ConstructionScript)

(fn UpdateRespawPoint
  (params (NewRespawPoint :type Transform) (CheckpointRef :type BP%20Checkpoint%20Object%20Reference))
  (Utilities|FlowControl|Sequence
    (:then_0
      (if (Utilities|IsValid (Variables|Default|GetCurrentCheckpoint))
        (Default|BacktoNormal (Variables|Default|GetCurrentCheckpoint))))
    (:then_1
      (Variables|Default|SetRespawPoint NewRespawPoint)
      (Variables|Default|SetCurrentCheckpoint CheckpointRef))))